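; BP_CamerInput is a trigger volume that pulls the third-person camera in close while the player is inside it.
; Box overlap stores the BP_ThirdPersonCharacter1 and sets a ShiftCamera flag, which any actor's end overlap clears.
; Tick uses that flag to drive the player's CameraBoom arm length between close and far targets through FInterpTo, with no interp speed set.
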(event OnComponentBeginOverlap(BoxCollider)
  (params (OverlappedComponent :type Primitive%20Component%20Object%20Reference) (OtherActor :type Actor%20Object%20Reference) (OtherComp :type Primitive%20Component%20Object%20Reference) (OtherBodyIndex :type Integer) (bFromSweep :type Boolean) (SweepResult :type Hit%20Result%20Structure%20%28by%20ref%29))
  (bind _asbp_third_person_character_1 (Utilities|Casting|CastToBP_ThirdPersonCharacter1 OtherActor))
  (Variables|Default|SetPlayer _asbp_third_person_character_1)
  (Variables|Default|SetShiftCamera true))

(event OnComponentEndOverlap(BoxCollider)
  (params (OverlappedComponent :type Primitive%20Component%20Object%20Reference) (OtherActor :type Actor%20Object%20Reference) (OtherComp :type Primitive%20Component%20Object%20Reference) (OtherBodyIndex :type Integer))
  (Variables|Default|SetShiftCamera false))

(event EventTick
  (params (DeltaSeconds :type Float%20%28single-precision%29))
  (bind _player (Variables|Default|GetPlayer))
  (bind _player_2 (Variables|Default|GetPlayer))
  (bind _cameraboom (Variables|/Game/ThirdPerson/Blueprints/BP_ThirdPersonCharacter1.BP_ThirdPersonCharacter1_C|GetCameraBoom _player))
  (bind _cameraboom_2 (Variables|/Game/ThirdPerson/Blueprints/BP_ThirdPersonCharacter1.BP_ThirdPersonCharacter1_C|GetCameraBoom _player_2))
  (if (Variables|Default|GetShiftCamera)
    (Utilities|IsValid _player_2
      (:Is%20Valid
        (Variables|/Script/Engine.SpringArmComponent|SetTargetArmLength _cameraboom_2 (Math|Interpolation|FInterpTo (Variables|/Script/Engine.SpringArmComponent|GetTargetArmLength _cameraboom_2) 8e+01 (Utilities|Time|GetWorldDeltaSeconds) 0.0))))
    (else
      (Utilities|IsValid _player
        (:Is%20Valid
          (Variables|/Script/Engine.SpringArmComponent|SetTargetArmLength _cameraboom (Math|Interpolation|FInterpTo (Variables|/Script/Engine.SpringArmComponent|GetTargetArmLength _cameraboom) 5e+02 (Utilities|Time|GetWorldDeltaSeconds) 0.0)))))))

(fn ConstructionScript)