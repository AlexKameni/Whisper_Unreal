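; Downward transport tube actor that changes the player's gravity while they travel through it.
; Entering the Box sends the tube's Gravity through BPI_Interaction's TransportTubeMessage with Up false.
; Touching GroundBox, or leaving the Box when Exit is set, sends a fixed gravity value instead.
; The construction script applies a dynamic holographic refraction material to the cylinder, driven by speed, brightness and color variables.
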(event OnComponentBeginOverlap(Box)
  (params (OverlappedComponent :type Primitive%20Component%20Object%20Reference) (OtherActor :type Actor%20Object%20Reference) (OtherComp :type Primitive%20Component%20Object%20Reference) (OtherBodyIndex :type Integer) (bFromSweep :type Boolean) (SweepResult :type Hit%20Result%20Structure%20%28by%20ref%29))
  (if (Actor|ActorHasTag OtherActor "Player")
    (if (Utilities|DoesObjectImplementInterface OtherActor "/Game/Blueprints/TransportTube/BPI_Interaction.BPI_Interaction_C")
      (Class|BPIInteraction|TransportTube(Message) OtherActor (Variables|Default|GetGravity) false))))

(event OnComponentEndOverlap(Box)
  (params (OverlappedComponent :type Primitive%20Component%20Object%20Reference) (OtherActor :type Actor%20Object%20Reference) (OtherComp :type Primitive%20Component%20Object%20Reference) (OtherBodyIndex :type Integer))
  (if (Variables|Default|GetExit)
    (if (Actor|ActorHasTag OtherActor "Player")
      (if (Utilities|DoesObjectImplementInterface OtherActor "/Game/Blueprints/TransportTube/BPI_Interaction.BPI_Interaction_C")
        (Class|BPIInteraction|TransportTube(Message) OtherActor 3.0 false)))))

(event OnComponentBeginOverlap(GroundBox)
  (params (OverlappedComponent :type Primitive%20Component%20Object%20Reference) (OtherActor :type Actor%20Object%20Reference) (OtherComp :type Primitive%20Component%20Object%20Reference) (OtherBodyIndex :type Integer) (bFromSweep :type Boolean) (SweepResult :type Hit%20Result%20Structure%20%28by%20ref%29))
  (if (Actor|ActorHasTag OtherActor "Player")
    (if (Utilities|DoesObjectImplementInterface OtherActor "/Game/Blueprints/TransportTube/BPI_Interaction.BPI_Interaction_C")
      (Class|BPIInteraction|TransportTube(Message) OtherActor 3.0 false))))

(fn ConstructionScript
  (bind _returnvalue (Rendering|Material|CreateDynamicMaterialInstance "/Game/SuperGrid/StarterPack/Materials/Base/M_SuperGrid_HoloRefract.M_SuperGrid_HoloRefract" "None" "None" :!class /Script/Engine.KismetMaterialLibrary))
  (Rendering|Material|SetScalarParameterValue _returnvalue "SpeedY_A" (Variables|Default|GetSpeed) :!class /Script/Engine.MaterialInstanceDynamic)
  (Rendering|Material|SetScalarParameterValue _returnvalue "Brightness" (Variables|Default|GetBrightness) :!class /Script/Engine.MaterialInstanceDynamic)
  (Rendering|Material|SetVectorParameterValue _returnvalue "PrimaryColor" (Variables|Default|GetPrimaryColor) :!class /Script/Engine.MaterialInstanceDynamic)
  (Rendering|Material|SetVectorParameterValue _returnvalue "SecondaryColor" (Variables|Default|GetSecondaryColor) :!class /Script/Engine.MaterialInstanceDynamic)
  (Rendering|Material|SetMaterial (Variables|Default|GetSuperGrid_CylinderFull) 0 _returnvalue))